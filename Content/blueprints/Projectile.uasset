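; Projectile actor that deals damage on overlap and plays laser impact effects.
; On overlap, it sends a health message to IDamageable actors, skipping those tagged Friendly, which it passes through without effect.
; Damaged targets and non-damageable actors both trigger an attached hit sound with random pitch and a spark emitter, then the projectile destroys itself.
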(event `self.ReceiveActorBeginOverlap`
  (params (OtherActor :type "Actor Object Reference"))
  (bind (_returnvalue_location _returnvalue_rotation) (`KismetMathLibrary.BreakTransform` (`self.GetTransform`)))
  (if (`KismetSystemLibrary.DoesImplementInterface` OtherActor "/Game/blueprints/iDamageable.iDamageable_C")
    (if (not (`self.ActorHasTag` OtherActor "Friendly"))
      (message `/Game/blueprints/iDamageable.AffectHealth` OtherActor (`self.Damage`))
      (`GameplayStatics.SpawnSoundAttached` "/Game/Audio/LaserHit.LaserHit" (`self.ProjectileCollision`) "None" (0.0 0.0 0.0) (struct) "KeepRelativeOffset" false 0.2 (`KismetMathLibrary.RandomFloatInRange` 0.85 1.1) 0.0 null null :!label _label)
      (`GameplayStatics.SpawnEmitterAtLocation` "/Game/StarterContent/Particles/LaserSparks.LaserSparks" _returnvalue_location _returnvalue_rotation)
      (`self.K2_DestroyActor`))
    (else
      (goto _label))))

(fn `UserConstructionScript`)